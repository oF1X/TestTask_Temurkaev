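; BP_Sphere is an actor whose sphere animates opacity, height and glow through four custom events.
; On BeginPlay it creates a dynamic material instance, which timelines drive through opacity and emission parameters.
; One event pair plays or reverses a 300-unit vertical lerp, with ShowAnimPlayRate scaling its alpha, alongside separate opacity timelines.
; The other pair sets full opacity and plays or reverses emission, skipping updates at or above MaxEmissive.
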(event `self.ReceiveBeginPlay`
  (bind _returnvalue (`PrimitiveComponent.CreateDynamicMaterialInstance` (`self.Sphere`) 0 "/Game/Task01/Sphere_Material.Sphere_Material" "None"))
  (set `self.SphereMaterial` _returnvalue))

(event `0_CustomEvent`
  (bind _startpoint (`self.StartPoint`))
  (bind (_returnvalue_x _returnvalue_y _returnvalue_z) (`KismetMathLibrary.BreakVector` (`SceneComponent.K2_GetComponentLocation` (`self.Sphere`))))
  (`|ExecutionSequence`
    (:`then_0`
      (bind (_direction _opacity) (`Timeline|ChangeOpacity` :!via `PlayFromStart`)
        (:`Update`
          (`MaterialInstanceDynamic.SetScalarParameterValue` (`self.SphereMaterial`) "SphereOpacity" _opacity))))
    (:`then_1`
      (set `self.StartPoint` _returnvalue_z)
      (bind (_direction_2 _movement) (`Timeline|MovementVertical` :!via `PlayFromStart` :!label _label)
        (:`Update`
          (`SceneComponent.K2_SetWorldLocation` (`self.Sphere`) (`KismetMathLibrary.MakeVector` _returnvalue_x _returnvalue_y (`KismetMathLibrary.Lerp` _startpoint (+ _startpoint 300.0) (* _movement (`self.ShowAnimPlayRate`)))) false false))))))

(event `1_CustomEvent`
  (bind (_returnvalue_x _returnvalue_y _returnvalue_z) (`KismetMathLibrary.BreakVector` (`SceneComponent.K2_GetComponentLocation` (`self.Sphere`))))
  (`|ExecutionSequence`
    (:`then_0`
      (set `self.StartPoint` (- _returnvalue_z 300.0))
      (goto _label :!via `ReverseFromEnd`))
    (:`then_1`
      (bind (_direction _opacity) (`Timeline|ReChangeOpacity`)
        (:`Update`
          (`MaterialInstanceDynamic.SetScalarParameterValue` (`self.SphereMaterial`) "SphereOpacity" _opacity))))))

(event `2_CustomEvent`
  (`MaterialInstanceDynamic.SetScalarParameterValue` (`self.SphereMaterial`) "SphereOpacity" 1.0)
  (bind (_direction _emission) (`Timeline|EmissinChange` :!via `PlayFromStart` :!label _label_2)
    (:`Update`
      (if (not (>= _emission (`self.MaxEmissive`)))
        (`MaterialInstanceDynamic.SetScalarParameterValue` (`self.SphereMaterial`) "SphereEmission" _emission)))))

(event `3_CustomEvent`
  (`MaterialInstanceDynamic.SetScalarParameterValue` (`self.SphereMaterial`) "SphereOpacity" 1.0)
  (goto _label_2 :!via `ReverseFromEnd`))

(fn `UserConstructionScript`)