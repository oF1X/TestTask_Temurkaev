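; BP_TestEffect is a light fixture that fades one of its three spot lights or its point light in and out.
; ShowLight and HideLIght play or reverse the LightUp timeline, which drives the light selected by EffectName.
; Speed scales the lerp alpha toward intensities cached at construction, so it affects brightness rather than timeline rate.
; The construction script's Sphere flag swaps sphere and cube meshes and toggles visibility between PointLight and SpotLight1/2.
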(event `ShowLight`
  (params (Speed :type "Float (double-precision)") (EffectName :type Name))
  (set `self.Speed` Speed)
  (set `self.Effect Name` EffectName)
  (bind (_direction _light) (`Timeline|LightUp` :!via `PlayFromStart` :!label _label)
    (:`Update`
      (switch `name` (`self.Effect Name`)
        (:`SpotLight`
          (`self.NewFunction` _light (`self.LightIntensity`) (`self.SpotLight`)))
        (:`SpotLight1`
          (`self.NewFunction` _light (`self.1LightIntensity`) (`self.SpotLight1`)))
        (:`SpotLight2`
          (`self.NewFunction` _light (`self.2LightIntensity`) (`self.SpotLight2`)))
        (:`PointLight`
          (`self.NewFunction` _light (`self.PointIntensity`) (`self.PointLight`)))))))

(event `HideLIght`
  (params (Speed :type "Float (double-precision)") (EffectName :type Name))
  (set `self.Speed` Speed)
  (set `self.Effect Name` EffectName)
  (goto _label :!via `ReverseFromEnd`))

(fn `NewFunction`
  (params (Alpha :type "Float (double-precision)") (B_Intensity :type "Float (double-precision)") (Target :type "LightComponent Object Reference"))
  (`LightComponent.SetIntensity` Target (`KismetMathLibrary.Lerp` 0.0 B_Intensity (* Alpha (/ (`self.Speed`) 10.0)))))

(fn `UserConstructionScript`
  (bind _staticmesh (`self.StaticMesh`))
  (bind _spotlight2 (`self.SpotLight2`))
  (bind _pointlight (`self.PointLight`))
  (set `self.PointIntensity` (`LightComponentBase.Intensity` (`self.PointLight`)))
  (set `self.2LightIntensity` (`LightComponentBase.Intensity` (`self.SpotLight2`)))
  (set `self.1LightIntensity` (`LightComponentBase.Intensity` (`self.SpotLight1`)))
  (set `self.LightIntensity` (`LightComponentBase.Intensity` (`self.SpotLight`)))
  (if (`self.Sphere ?`)
    (`StaticMeshComponent.SetStaticMesh` _staticmesh "/Engine/BasicShapes/Sphere.Sphere")
    (`SceneComponent.SetVisibility` _spotlight2 false false)
    (`SceneComponent.SetVisibility` (`self.SpotLight1`) false false)
    (`SceneComponent.SetVisibility` _pointlight true false)
    (else
      (`StaticMeshComponent.SetStaticMesh` _staticmesh "/Engine/BasicShapes/Cube.Cube")
      (`SceneComponent.SetVisibility` _spotlight2 true false)
      (`SceneComponent.SetVisibility` (`self.SpotLight1`) true false)
      (`SceneComponent.SetVisibility` _pointlight false false))))